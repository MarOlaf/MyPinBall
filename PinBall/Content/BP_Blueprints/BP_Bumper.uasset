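; BP_Bumper is a pinball pop bumper that knocks the ball away and awards score on contact.
; A capsule overlap with BP_BallSphere applies a radial velocity-change impulse, adds score through GameMode_PinBall and plays a hit sound.
; A timeline animates the mechanism, spotlight, and logo color and emissive glow on a dynamic material created in the Construction Script.
; Tuning values come from a BP_BumperManager found at BeginPlay.
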(event OnComponentBeginOverlap(Capsule)
  (params (OverlappedComponent :type Primitive%20Component%20Object%20Reference) (OtherActor :type Actor%20Object%20Reference) (OtherComp :type Primitive%20Component%20Object%20Reference) (OtherBodyIndex :type Integer) (bFromSweep :type Boolean) (SweepResult :type Hit%20Result%20Structure%20%28by%20ref%29))
  (bind _asbp_ball_sphere (Utilities|Casting|CastToBP_BallSphere OtherActor))
  (CallFunction|Bump _asbp_ball_sphere))

(event Custom|Bump
  (params (Ball :type BP%20Ball%20Sphere%20Object%20Reference%20%28by%20ref%29))
  (bind _bumpertop (Variables|Default|GetBumperTop))
  (bind _bp_bumpermanager (Variables|Default|GetBP_BumperManager))
  ;[1 1 1] BumpAction
  (Utilities|IsValid Ball
    (:Is%20Valid
      (Physics|AddImpulse (Variables|/Game/BP_Blueprints/BP_BallSphere.BP_BallSphere_C|GetBall Ball) (* (Math|Vector|GetUnitDirection(Vector) (Transformation|GetActorLocation) (Transformation|GetActorLocation Ball)) (Variables|/Game/BP_Blueprints/BP_BumperManager.BP_BumperManager_C|GetIntensityBump _bp_bumpermanager)) "None" true)
      ;[1 1 1] Add Score
      (bind _asgame_mode_pin_ball (Utilities|Casting|CastToGameMode_PinBall (Game|GetGameMode))
        (:then
          (bind _newscore (Default|AddScore _asgame_mode_pin_ball (Variables|/Game/BP_Blueprints/BP_BumperManager.BP_BumperManager_C|GetScoreToAdd _bp_bumpermanager)))
          (Development|PrintString (Utilities|String|ToString(Float) _newscore)))
        (:CastFailed
          (Development|PrintString "GameMode Warning: Failed cast to GameMode_PinBall")))
      ;[1 1 1] BumpFX
      (Audio|SpawnSoundAttached "/Game/Assets/Bumper/S_BumperHit.S_BumperHit" (Variables|Default|GetBumper) "None" "0, 0, 0" "0, 0, 0" "KeepRelativeOffset" false 1.0 1.0 0.0 0 0)
      (bind (_direction _bumpalpha _lightalpha) (Timeline|BumpLerp PlayFromStart)
        (:Update
          (Transformation|SetRelativeLocation (Variables|Default|GetBumper_Mechanism) (Math|Vector|Lerp(Vector) "0, 0, 0" "0, 0,-65.000000" _bumpalpha) false false)
          (Rendering|Components|Light|SetIntensity (Variables|Default|GetSpotLight) (Math|Float|Lerp 0.0 (Variables|/Game/BP_Blueprints/BP_BumperManager.BP_BumperManager_C|GetIntensitiyLight _bp_bumpermanager) _lightalpha))
          (Rendering|Material|SetScalarParameterValue _bumpertop "EmissiveBoostLogo" (Math|Float|Lerp 1.0 (Variables|/Game/BP_Blueprints/BP_BumperManager.BP_BumperManager_C|GetEmissiveBoost _bp_bumpermanager) _bumpalpha) :!class /Script/Engine.MaterialInstanceDynamic)
          (Rendering|Material|SetVectorParameterValue _bumpertop "LogoColor" (Math|Color|Lerp(LinearColor) (Variables|/Game/BP_Blueprints/BP_BumperManager.BP_BumperManager_C|GetColor_0 _bp_bumpermanager) (Variables|/Game/BP_Blueprints/BP_BumperManager.BP_BumperManager_C|GetColor_1 _bp_bumpermanager) _bumpalpha) :!class /Script/Engine.MaterialInstanceDynamic))))))

(event EventBeginPlay
  (bind _returnvalue (Actor|GetActorOfClass "/Game/BP_Blueprints/BP_BumperManager.BP_BumperManager_C"))
  (bind _output_get (Variables|Default|SetBP_BumperManager _returnvalue))
  (Rendering|Material|SetVectorParameterValue (Variables|Default|GetBumperTop) "LogoColor" (Variables|/Game/BP_Blueprints/BP_BumperManager.BP_BumperManager_C|GetColor_0 _output_get) :!class /Script/Engine.MaterialInstanceDynamic))

(fn ConstructionScript
  (bind _returnvalue (Rendering|Material|CreateDynamicMaterialInstance (Variables|Default|GetBumper) 1 "/Game/Assets/Bumper/M_PopBumper_Inst.M_PopBumper_Inst" "None" :!class /Script/Engine.PrimitiveComponent))
  (Variables|Default|SetBumperTop _returnvalue))