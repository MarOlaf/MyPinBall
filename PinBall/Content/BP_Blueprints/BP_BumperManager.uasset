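; BP_BumperManager is a configuration Blueprint that resolves the initial and bump colors for bumpers, judging by its names.
; Its Construction Script switches on two color selections, ColorInitial and ColorBump, copying the matching preset color variable into Color0 and Color1 respectively.
; Both selections share the same five-color palette, and the Event Graph holds no runtime logic.
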(event EventBeginPlay)

(fn ConstructionScript
  (Utilities|FlowControl|Sequence
    (:then_0
      (switch Utilities|FlowControl|Switch|SwitchonColor0 (Variables|Default|GetColorInitial)
        (:NewEnumerator0
          (Variables|Default|SetColor_0 (Variables|Default|GetColor_2)))
        (:NewEnumerator4
          (Variables|Default|SetColor_0 (Variables|Default|GetColor_6)))
        (:NewEnumerator1
          (Variables|Default|SetColor_0 (Variables|Default|GetColor_4)))
        (:NewEnumerator2
          (Variables|Default|SetColor_0 (Variables|Default|GetColor_5)))
        (:NewEnumerator3
          (Variables|Default|SetColor_0 (Variables|Default|GetColor_3)))))
    (:then_1
      (switch Utilities|FlowControl|Switch|SwitchonColor1 (Variables|Default|GetColorBump)
        (:NewEnumerator0
          (Variables|Default|SetColor_1 (Variables|Default|GetColor_2)))
        (:NewEnumerator4
          (Variables|Default|SetColor_1 (Variables|Default|GetColor_6)))
        (:NewEnumerator1
          (Variables|Default|SetColor_1 (Variables|Default|GetColor_4)))
        (:NewEnumerator2
          (Variables|Default|SetColor_1 (Variables|Default|GetColor_5)))
        (:NewEnumerator3
          (Variables|Default|SetColor_1 (Variables|Default|GetColor_3)))))))