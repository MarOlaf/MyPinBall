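; BP_BallSphere is a physics ball actor with custom gravity and a stick-to-surface force.
; It enables physics on the Ball component shortly after BeginPlay.
; While simulating, each Tick applies GravityBall as a delta-time-scaled velocity impulse.
; A downward line trace from the actor finds the surface below, and a second impulse scaled by StickynessBall pushes the ball against that surface's normal.
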(event EventBeginPlay
  (Utilities|FlowControl|Delay 0.2)
  (Physics|SetSimulatePhysics (Variables|Default|GetBall) true))

(event EventTick
  (params (DeltaSeconds :type Float%20%28single-precision%29))
  (bind _returnvalue (Transformation|GetActorLocation))
  (if (Physics|IsSimulatingPhysics (Variables|Default|GetBall) "None")
    (Physics|AddImpulse (Variables|Default|GetBall) (* DeltaSeconds (Variables|Default|GetGravityBall)) "None" true)
    (bind _outhit (Collision|LineTraceByChannel _returnvalue (- _returnvalue "0,0,500.000000") "TraceTypeQuery1" false 0 "None"))
    (Physics|AddImpulse (Variables|Default|GetBall) (* (* (.ImpactNormal (Collision|BreakHitResult _outhit)) -1.0) (* (Variables|Default|GetStickynessBall) DeltaSeconds)) "None" true)))

(fn ConstructionScript)