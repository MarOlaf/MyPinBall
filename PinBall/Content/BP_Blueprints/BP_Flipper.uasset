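; BP_Flipper is a left or right flipper, likely pinball-style, that swings between a rest and a raised rotation.
; The construction script picks mirrored start and end rotations from FlipType, applies the start one, and mirrors the mesh with negative X scale for Left.
; Flip and Flop events use MoveComponentTo to rotate the Flipper component to the end or start rotation over TimeFlip.
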(event Custom|Flip
  (Components|MoveComponentTo (Variables|Default|GetFlipper) "0, 0, 0" (Variables|Default|GetRotationEnd) false false (Variables|Default|GetTimeFlip) false))

(event Custom|Flop
  (Components|MoveComponentTo (Variables|Default|GetFlipper) "0, 0, 0" (Variables|Default|GetRotationStart) false false (Variables|Default|GetTimeFlip) false))

(fn ConstructionScript
  (bind _fliptype (Variables|Default|GetFlipType))
  (Variables|Default|SetRotationStart (Utilities|Select :Index _fliptype :NewEnumerator0 "0,20.000000, 0" :NewEnumerator1 "0,-20.000000, 0"))
  (Variables|Default|SetRotationEnd (Utilities|Select :Index _fliptype :NewEnumerator0 "0,-40.000000, 0" :NewEnumerator1 "0,40.000000, 0"))
  (Transformation|SetRelativeRotation (Variables|Default|GetFlipper) (Variables|Default|GetRotationStart) false false)
  (switch Utilities|FlowControl|Switch|SwitchonFlipType (Variables|Default|GetFlipType)
    (:NewEnumerator0
      (Transformation|SetRelativeScale3D (Variables|Default|GetFlipper) "-1.000000,1.000000,1.000000"))))