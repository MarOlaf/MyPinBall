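; BP_Plunger is a ball plunger actor with pull and release events that move its mesh.
; PullPlunger plays a timeline that lerps the mesh's relative location from zero toward DistancePull.
; ReleasePlunger stops the timeline and eases the mesh back to zero over TimePush with MoveComponentTo.
; GetBallSpawnLocation converts the LocationBall offset to world space through the actor transform.
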(event Custom|Pull%20Plunger
  (bind _newtrack_0 (Timeline|Test PlayFromStart)
    (:Update
      (Transformation|SetRelativeLocation (Variables|Default|GetSM_Plunger) (Math|Vector|Lerp(Vector) "0, 0, 0" (Variables|Default|GetDistancePull) _newtrack_0) false false))))

(event Custom|Release%20Plunger
  (Utilities|FlowControl|Sequence
    (:then_0
      (bind _newtrack_0 (Timeline|Test Stop)
        (:Update
          (Transformation|SetRelativeLocation (Variables|Default|GetSM_Plunger) (Math|Vector|Lerp(Vector) "0, 0, 0" (Variables|Default|GetDistancePull) _newtrack_0) false false))))
    (:then_1
      (Components|MoveComponentTo (Variables|Default|GetSM_Plunger) "0, 0, 0" "0, 0, 0" false true (Variables|Default|GetTimePush) false))))

(fn ConstructionScript)

(fn GetBallSpawnLocation
  (params (test :type Vector))
  (return (Math|Transform|TransformLocation (Transformation|GetActorTransform) (Variables|Default|GetLocationBall))))